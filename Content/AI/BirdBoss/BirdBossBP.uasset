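; Bird boss pawn that sets its max health at start and relies on a behavior tree for combat.
; Tick caches the blackboard state and stops the brain on death.
; Notify functions implement attacks: wing overlaps launch players outward, beak overlap deals damage and clears peck availability, and bug spawning places a random-sized group at navigable points ahead.
; Debug prints and a debug sphere remain active.
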(event EventTick
  (params (DeltaSeconds :type Float%20%28single-precision%29))
  (bind _returnvalue (Class|EnemyCharacter|GetHealthPoint))
  (Development|PrintString (Utilities|String|ToString(Float) _returnvalue))
  (bind _returnvalue_2 (AI|GetAIController self))
  (Variables|Default|SetAIController _returnvalue_2)
  (Variables|Default|SetMainState (Utilities|Enum|ByteToEnumEBirdBossState (Class|BlackboardComponent|GetValueasEnum (AI|GetBlackboard _returnvalue_2) (Variables|Default|GetState))))
  (bind _returnvalue_3 (Class|EnemyCharacter|GetBDead))
  (if _returnvalue_3
    (AI|Logic|StopLogic (Variables|/Script/AIModule.AIController|GetBrainComponent (Variables|Default|GetAIController)) "dead")))

(event EventBeginPlay
  (Class|EnemyCharacter|SetMaxHealthPoint 4e+02))

(fn ConstructionScript)

(fn WindblastNotify
  (Development|PrintString "Windblast" true true "(R=0.540000,G=0.034845,B=0.099496,A=1.000000)")
  (for _array_element (Collision|GetOverlappingActors (Variables|Default|GetCoupAile) "/Script/DarklightProject.DarklightProjectCharacter" :!class /Script/Engine.PrimitiveComponent)
    (bind _asdarklight_project_character (Utilities|Casting|CastToDarklightProjectCharacter _array_element))
    (Character|LaunchCharacter _asdarklight_project_character (* (Math|Vector|Normalize (Math|Vector|MakeVector (.X (Math|Vector|BreakVector (- (Transformation|GetActorLocation _asdarklight_project_character) (Transformation|GetActorLocation)))) (.Y (Math|Vector|BreakVector (- (Transformation|GetActorLocation _asdarklight_project_character) (Transformation|GetActorLocation)))) 0.0)) (Variables|Default|GetLaunchForce)) false false))
  (for _array_element_2 (Collision|GetOverlappingActors (Variables|Default|GetCoupAile2) "/Script/DarklightProject.DarklightProjectCharacter" :!class /Script/Engine.PrimitiveComponent)
    (bind _asdarklight_project_character_2 (Utilities|Casting|CastToDarklightProjectCharacter _array_element_2))
    (Character|LaunchCharacter _asdarklight_project_character_2 (* (Math|Vector|Normalize (Math|Vector|MakeVector (.X (Math|Vector|BreakVector (- (Transformation|GetActorLocation _asdarklight_project_character_2) (Transformation|GetActorLocation)))) (.Y (Math|Vector|BreakVector (- (Transformation|GetActorLocation _asdarklight_project_character_2) (Transformation|GetActorLocation)))) 0.0)) (Variables|Default|GetLaunchForce)) false false))
  (return true))

(fn PeckNotify
  (Development|PrintString "Peck" true true "(R=0.545000,G=0.011354,B=0.011354,A=1.000000)")
  (for _array_element (Collision|GetOverlappingActors (Variables|Default|GetAttackBec) "/Script/DarklightProject.DarklightProjectCharacter" :!class /Script/Engine.PrimitiveComponent)
    (Utilities|FlowControl|DoOnce false
      (:Completed
        (bind _asdarklight_project_character (Utilities|Casting|CastToDarklightProjectCharacter _array_element))
        (Game|Damage|ApplyDamage _asdarklight_project_character 1e+01 0 0))))
  (AI|Components|Blackboard|SetValueasBool (AI|GetBlackboard (Variables|Default|GetAIController)) (Variables|Default|GetavailablePeck) false)
  (return true))

(fn SpawnbugsNotify
  (bind _returnvalue (Transformation|GetActorForwardVector))
  (bind _returnvalue_2 (Transformation|GetActorLocation))
  (bind _returnvalue_3 (* _returnvalue 7e+02))
  (bind _returnvalue_4 (+ _returnvalue_2 _returnvalue_3))
  (Development|PrintString "Spawnbugs" true true "(R=0.650000,G=0.027083,B=0.027083,A=1.000000)")
  (Variables|Default|SetCompteur 0.0)
  (Variables|Default|SetmaxEnemy (Math|Conversions|ToFloat(Integer) (Math|Random|RandomIntegerinRange 4 8)))
  (if (< (Variables|Default|GetCompteur) (Variables|Default|GetMaxEnemy)) :!label _label
    (Rendering|Debug|DrawDebugSphere _returnvalue_4 1e+03 12 "(R=0.000000,G=0.276372,B=1.000000,A=1.000000)" 99.0 0.0)
    (AI|SpawnAIFromClass "/Game/AI/BugEnemySpawn_Character.BugEnemySpawn_Character_C" 0 (Class|NavigationSystem|GetRandomPointinNavigableRadius _returnvalue_4 8e+02) "0, 0, 0" false)
    (bind _result (Math|Float|IncrementFloat (Variables|Default|GetCompteur))
      (:%20%20
        (Variables|Default|SetCompteur _result)
        (goto _label)))
    (else
      (return true))))