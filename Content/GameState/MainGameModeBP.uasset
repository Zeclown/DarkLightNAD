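; Main game mode Blueprint that handles HUD setup, player death, checkpoint saves and the first-load intro.
; BeginPlay adds the in-game overlay and a BlackIn widget, then focuses the game viewport.
; Death disables input and shows a delayed blackout before deferring to the parent handler, while checkpoint saves call the parent and show a save indicator.
; On first load it plays a level sequence with input briefly disabled.
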(event EventBeginPlay
  (bind _returnvalue (UserInterface|CreateWidget "/Game/UI/InGameOverlay.InGameOverlay_C" (Game|GetPlayerController 0)))
  (UserInterface|Viewport|AddtoViewport _returnvalue 0)
  (bind _returnvalue_2 (UserInterface|CreateWidget "/Game/UI/BlackIn.BlackIn_C"))
  (UserInterface|Viewport|AddtoViewport _returnvalue_2 0)
  (Class|WidgetBlueprintLibrary|SetFocustoGameViewport))

(event EventSaveCheckpoint
  (params (CheckPoint :type Check%20Point%20Plant%20Object%20Reference))
  (|CallParentFunction CheckPoint)
  (bind _returnvalue (UserInterface|CreateWidget "/Game/UI/SaveInProgress.SaveInProgress_C"))
  (UserInterface|Viewport|AddtoViewport _returnvalue 0))

(event EventOnGameLoaded
  (bind _returnvalue (Game|GetPlayerController 0))
  (if (Variables|Default|GetbFirstLoad)
    (bind _returnvalue_2 (Sequencer|Player|CreateLevelSequencePlayer "/Game/Sandy/sequencetest.sequencetest"))
    (Audio|Components|Audio|Play _returnvalue_2)
    (Input|DisableInput _returnvalue _returnvalue)
    (Utilities|FlowControl|Delay 3.0)
    (Input|EnableInput _returnvalue _returnvalue)))

(event EventHandlePlayerDeath
  (bind _returnvalue (Game|GetPlayerController 0))
  (bind _returnvalue_2 (Game|GetPlayerController 0))
  (Input|DisableInput _returnvalue_2 _returnvalue_2)
  (Utilities|FlowControl|Delay 3.0)
  (bind _returnvalue_3 (UserInterface|CreateWidget "/Game/UI/Blackout.Blackout_C"))
  (UserInterface|Viewport|AddtoViewport _returnvalue_3 0)
  (Utilities|FlowControl|Delay 3.0)
  (Input|EnableInput _returnvalue _returnvalue)
  (|CallParentFunction))

(fn ConstructionScript)