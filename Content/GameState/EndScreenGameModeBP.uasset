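; End screen game mode that shows score-entry UI when a score is submitted.
; SubmitScore stores the highscore flag, but its branch is fixed to true, so it always creates the NewHighscore widget and never the Leaderboard.
; It adds the widget to the viewport and gives keyboard focus to the parent of its first character field.
; ReceiveName only forwards the name to the parent implementation.
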(event EventBeginPlay)

(event EventTick
  (params (DeltaSeconds :type Float%20%28single-precision%29)))

(event EventSubmitScore
  (params (isHighscore :type Boolean))
  (Variables|Default|SetbNewHighscore isHighscore)
  (if true
    (bind _returnvalue (UserInterface|CreateWidget "/Game/UI/NewHighscore.NewHighscore_C"))
    (Variables|Default|SetCurrentWidget _returnvalue)
    (else
      (bind _returnvalue_2 (UserInterface|CreateWidget "/Game/UI/Leaderboard.Leaderboard_C"))
      (Variables|Default|SetCurrentWidget _returnvalue_2)))
  (UserInterface|Viewport|AddtoViewport (Variables|Default|GetCurrentWidget) 0)
  (bind _asnew_highscore (Utilities|Casting|CastToNewHighscore (Variables|Default|GetCurrentWidget)))
  (Widget|SetKeyboardFocus (Widget|GetParent (Variables|/Game/UI/NewHighscore.NewHighscore_C|GetFirstChar _asnew_highscore))))

(fn ConstructionScript)

(fn ReceiveName
  (params (Name :type String))
  (bind _returnvalue (|CallParentFunction Name))
  (return _returnvalue))